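; Player controller for SirKnight that handles mouse clicks on room cells and provides click debugging.
; BeginPlay shows the cursor, sets Game and UI input, and adds a DebugScreen widget to the viewport.
; Left click traces the Visibility channel under the cursor and shows the hit actor's name on the widget for a second.
; A hit BP_RoomCell also has its coordinate printed and its EventTargeted called.
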(event `Key|LeftMouseButton`
  (params (Key :type "Key Structure"))
  (bind (_hitresult _returnvalue) (`self.GetHitResultUnderCursorByChannel` "TraceTypeQuery1"))
  (bind _debug_screen (`self.Debug Screen`))
  (bind (_bblockinghit _binitialoverlap _time _distance _location _impactpoint _normal _impactnormal _physmat _hitactor) (`GameplayStatics.BreakHitResult` _hitresult))
  ;[1 1 1] [DEBUG] What object am I clicking on?
  (:`Pressed`
    (if _returnvalue
      (`|ExecutionSequence`
        (:`then_0`
          (set `/Game/UI/DebugScreen.Debug Text` (`KismetTextLibrary.Conv_StringToText` (`KismetSystemLibrary.GetDisplayName` _hitactor)) _debug_screen)
          (`KismetSystemLibrary.Delay` 1.0)
          (set `/Game/UI/DebugScreen.Debug Text` "" _debug_screen))
        (:`then_1`
          (bind _asbp_room_cell (cast `/Game/Blueprints/BP_RoomCell` _hitactor))
          (bind (_coordinate_x _coordinate_y) (`KismetMathLibrary.BreakVector2D` (`/Game/Blueprints/BP_RoomCell.Coordinate` _asbp_room_cell)))
          (`KismetSystemLibrary.PrintString` (`KismetStringLibrary.Concat_StrStr` "X: " (`KismetStringLibrary.Conv_DoubleToString` _coordinate_x) " || Y: " (`KismetStringLibrary.Conv_DoubleToString` _coordinate_y)) true true (struct :`G` 0.66 :`B` 1.0 :`A` 1.0) 1.0)
          (`/Game/Blueprints/BP_RoomCell.Event Targeted` _asbp_room_cell))))))

(event `self.ReceiveBeginPlay`
  (`|ExecutionSequence`
    (:`then_1`
      (set `self.bShowMouseCursor` true)
      (`WidgetBlueprintLibrary.SetInputMode_GameAndUIEx` null)
      (bind _returnvalue (`|CreateWidget` "/Game/UI/DebugScreen.DebugScreen_C" self "Text Block"))
      (bind _output_get (set `self.Debug Screen` _returnvalue))
      (`UserWidget.AddToViewport` _output_get 0))))

(fn `UserConstructionScript`)