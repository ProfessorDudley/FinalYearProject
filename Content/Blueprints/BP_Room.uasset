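; Grid-based room actor that builds its tile layout at BeginPlay and becomes the player's view target.
; It generates coordinates, pairs them with a layout (currently forced) into a RoomTemplate map of tile ID, location and other per-tile data.
; AddFloorTile then attaches static mesh components to FloorRoot by tile ID, skipping voids.
; TargetTiles spawns target markers on adjacent coordinates found through that map, and ClearTargets destroys them.
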(event `self.ReceiveBeginPlay`
  (`self.Build Room with Grid` (`self.Grid Size`))
  (`PlayerController.SetViewTargetWithBlend` (`GameplayStatics.GetPlayerController` 0) self 0.0 "VTBlend_Linear" 0.0 false))

(event `Build Room with Grid`
  (params (`Grid Size` :type Integer))
  (bind _grid_coordinates (`/Game/Core/Functions_Pathfinding.Generate Grid` `Grid Size`))
  (bind _output_get (set `self.Grid Coordinates` _grid_coordinates))
  (bind _layout (`/Game/Core/Functions_Pathfinding.Choose Layout` (`self.Room Layouts`) true 2))
  (for (_array_element _array_index) _output_get
    (bind _output (`|GetArrayItem` _layout _array_index))
    (`BlueprintMapLibrary.Map_Add` (`self.Room Template`) _array_element (make `/Game/Blueprints/Struct_RoomGrid` _output (select `int` _output :`0` null :`1` null :`2` null :!type "Object Class Reference") (`/Game/Core/Functions_Pathfinding.Coords -> Vector` _array_element 100.0) (and (!= _output 0) (!= _output 1)))))
  (for _array_element_2 _output_get
    (`self.Build Geometry` _array_element_2)))

(event `Build Geometry`
  (params (Coordinate :type "Vector2D Structure (by ref)"))
  (`self.Add Floor Tile` Coordinate))

(fn `Add Floor Tile`
  (params (Coordinate :type "Vector2D Structure (by ref)"))
  (bind _floor_root (`self.Floor Root`))
  (bind _value (`BlueprintMapLibrary.Map_Find` (`self.Room Template`) Coordinate))
  (bind _returnvalue (`KismetMathLibrary.Conv_VectorToTransform` (`.Location_40_FC40F80447BA76F5D9B2C285AE1F78EA` (break `/Game/Blueprints/Struct_RoomGrid` _value))))
  (switch `int` (break `/Game/Blueprints/Struct_RoomGrid` _value)
    (:`Default`
      (bind _returnvalue_2 (`AddComponent|NODE_AddStaticMeshComponent-5` :`bManualAttachment` true :`RelativeTransform` _returnvalue))
      (`SceneComponent.K2_AttachToComponent` _returnvalue_2 _floor_root "None" "KeepRelative" "KeepRelative" "KeepRelative" true)
      (`BlueprintMapLibrary.Map_Add` (`self.FloorTiles`) Coordinate _returnvalue_2))
    (:`0`
      (`KismetSystemLibrary.PrintString` "Void")
      (return))
    (:`1`
      (`KismetSystemLibrary.PrintString` "Wall")
      (bind _returnvalue_3 (`AddComponent|NODE_AddStaticMeshComponent-6` :`bManualAttachment` true :`RelativeTransform` _returnvalue))
      (`SceneComponent.K2_AttachToComponent` _returnvalue_3 _floor_root "None" "KeepRelative" "KeepRelative" "KeepRelative" true)))
  (return))

(fn `ClearTargets`
  (bind _targeted_tiles (`self.Targeted Tiles`))
  (for _array_element _targeted_tiles
    (`self.K2_DestroyActor` _array_element))
  (`KismetArrayLibrary.Array_Clear` _targeted_tiles))

(fn `TargetTiles`
  (params (DamageType :type "/Game/Blueprints/Enum_DamageTypes Enum" :default "NewEnumerator0") (Coordinate :type "Vector2D Structure"))
  (bind (_found_coordinates _coordinates) (`/Game/Core/Functions_Pathfinding.Get Multiple Adjacent Coordinates` Coordinate (`self.Grid Coordinates`) (`self.Room Template`)))
  (if _found_coordinates
    (for _array_element _coordinates
      (bind _returnvalue (`|SpawnActorFromClass` "/Game/Blueprints/TargetTile.TargetTile_C" (`KismetMathLibrary.MakeTransform` (+ (`/Game/Core/Functions_Pathfinding.Coords -> Vector` _array_element 100.0) (0.0 0.0 5.0))) "Undefined" "OverrideRootScale" null null))
      (`KismetArrayLibrary.Array_Add` (`self.Targeted Tiles`) _returnvalue))
    (else
      (`KismetSystemLibrary.PrintString` "Unable to find target tiles" true true (struct :`R` 1.0 :`A` 1.0)))))

(fn `UserConstructionScript`)