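; Pawn_SirKnight is a pawn Blueprint that holds a knight character's health, defence and attack stats.
; ApplyHealth, ApplyDefence and ApplyAttack each add a value to the current stat and clamp it between zero and its maximum.
; When health reaches zero, ApplyHealth calls the PlayerDeath event, which is empty in this graph.
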(event `Player Death`)

(fn `ApplyAttack`
  (params (Value :type Integer))
  (set `self.CurrentAttack` (`KismetMathLibrary.Clamp` (+ Value (`self.CurrentAttack`)) 0 (`self.MaxAttack`))))

(fn `ApplyDefence`
  (params (A :type Integer))
  (set `self.CurrentDefence` (`KismetMathLibrary.Clamp` (+ A (`self.CurrentDefence`)) 0 (`self.MaxDefence`))))

(fn `ApplyHealth`
  (params (Value :type Integer))
  (bind _output_get (set `self.CurrentHealth` (`KismetMathLibrary.Clamp` (+ Value (`self.CurrentHealth`)) 0 (`self.MaxHealth`))))
  (if (<= _output_get 0)
    (`self.Player Death`)))

(fn `UserConstructionScript`)