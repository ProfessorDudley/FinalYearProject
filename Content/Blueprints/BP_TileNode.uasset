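; BP_TileNode is a tile node Blueprint that animates a highlight on its plane when targeted.
; The Targeted event restarts a timeline that drives the "Targeted Intensity" scalar parameter on the Plane's materials.
; BeginPlay caches the GM_Munchkin game mode, which the live graph does not otherwise use.
; Disconnected leftover nodes would show TileScore in a debug tag widget or reset it to zero.
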(event `self.ReceiveBeginPlay`
  (set `self.Gamemode` (cast `/Game/Core/GM_Munchkin` (`GameplayStatics.GetGameMode`) :!pure true)))

(event `Targeted`
  (bind (_direction _scalar_value) (`Timeline|Timeline_0` :!via `PlayFromStart`)
    (:`Update`
      (`MeshComponent.SetScalarParameterValueOnMaterials` (`self.Plane`) "Targeted Intensity" _scalar_value))))

(fn `UserConstructionScript`)