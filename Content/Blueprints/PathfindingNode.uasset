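; PathfindingNode is a placeable tile node for pathfinding, with a static mesh, a box and a debug widget component.
; Clicking the mesh prints a test "Hello" message; BeginPlay, the box click and the construction script are empty.
; Unconnected logic would create a DebugTag widget showing the tile's score and reset that score to zero, but it never runs.
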(event `self.ReceiveBeginPlay`)

(event `self.Box.OnClicked`
  (params (TouchedComponent :type "PrimitiveComponent Object Reference") (ButtonPressed :type "Key Structure")))

(event `self.StaticMesh.OnClicked`
  (params (TouchedComponent :type "PrimitiveComponent Object Reference") (ButtonPressed :type "Key Structure"))
  (`KismetSystemLibrary.PrintString` "Hello"))

(fn `UserConstructionScript`)