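; Game mode for the Munchkin game that starts a new game on BeginPlay by streaming in the dungeon level, spawning the player and possessing it.
; The Sir Knight pawn spawns once, centered on a tile from the spawn coordinate, and is handed to PC_SirKnight for possession.
; Room creation, tile layout and camera switching remain as disconnected logic, alongside an older tile-grid spawn event that nothing here calls.
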(event `self.ReceiveBeginPlay`
  (`KismetSystemLibrary.PrintString` "Gamemode Intialised Successfully")
  (`self.Initialise NewGame`))

(event `Initialise NewGame`
  (`|ExecutionSequence`
    (:`then_0`
      (`GameplayStatics.LoadStreamLevel` "lvl_Dungeon" true)
      (`self.Spawn Player`)
      (`self.Possess Active Character`))))

(event `Spawn P`
  (bind __old__player_spawn (`self.[OLD] Player Spawn`))
  (`/Engine/EditorBlueprintResources/StandardMacros.IsValid` (`self.Player`) ; Check if the player already exists.
    (:`Is Valid`
      (`KismetSystemLibrary.PrintString` "The player already exists" true true (struct :`R` 0.060697 :`B` 1.0 :`A` 1.0)))
    (:`Is Not Valid`
      (bind _returnvalue (`|SpawnActorFromClass` "/Game/Blueprints/Pawn_SirKnight.Pawn_SirKnight_C" (`KismetMathLibrary.Conv_VectorToTransform` (+ (`self.K2_GetActorLocation` (`BlueprintMapLibrary.Map_Find` (`/Game/Blueprints/BP_Room.Tile Grid` (`self.Current Room`)) __old__player_spawn)) (50.0 50.0 100.0))) "Undefined" "OverrideRootScale" null __old__player_spawn self null))
      (set `self.Player` _returnvalue) ; Save the spawned player so we can track it/.
    )))

(event `CreateDungeon`
  (`GameplayStatics.LoadStreamLevel` (`self.DungeonLevel`) true))

(fn `Create New Room`
  (returns (Room :type "/Game/Blueprints/BP_Room Object Reference"))
  (locals (`Room Spawn Location` :type "Transform Structure")))

(fn `Possess Active Character`
  (bind _aspc_sir_knight (cast `/Game/Core/PC_SirKnight` (`GameplayStatics.GetPlayerController` 0) :!pure true))
  (bind _output_get (set `/Game/Core/PC_SirKnight.Active Player` (`self.Active Player`) _aspc_sir_knight))
  (`Controller.Possess` _aspc_sir_knight _output_get))

(fn `Room tiles`
  (returns (SpawnedTiles1 :type "Array of /Game/Blueprints/Tiles/BP_Tile Object Reference"))
  (locals (SpawnedTiles :type "Array of /Game/Blueprints/Tiles/BP_Tile Object Reference") (`[LOCAL] Layout` :type "Array of Integer")))

(fn `Spawn Player`
  (locals (`Player Spawn Coordinate` :type "Vector2D Structure" :default (5.0 3.0)))
  (`/Engine/EditorBlueprintResources/StandardMacros.IsValid` (`self.Active Player`)
    (:`Is Valid`
      (`KismetSystemLibrary.PrintString` "Failed to Spawn Player: Player already exists" true true (struct :`R` 1.0 :`G` 0.030725 :`B` 0.020778 :`A` 1.0)))
    (:`Is Not Valid`
      (bind _returnvalue (`/Game/Core/WorldGrid.Coordinates to Vector` (`local.Player Spawn Coordinate`) 100.0))
      (bind _returnvalue_2 (`|SpawnActorFromClass` "/Game/Blueprints/Pawn_SirKnight.Pawn_SirKnight_C" (`KismetMathLibrary.MakeTransform` (+ _returnvalue (50.0 50.0 100.0))) "Undefined" "OverrideRootScale" null (0.0 0.0) null null))
      (set `self.Active Player` _returnvalue_2))))

(fn `UserConstructionScript`)