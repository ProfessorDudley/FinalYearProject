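; Game mode for a turn-based strategy (TBS) game that bootstraps core manager actors and a debug HUD.
; On BeginPlay it spawns the TBS AI controller and room manager and stores references to both.
; It then creates a DebugScreen widget, adds it to the viewport, and appends a stat display showing the room manager's name to its statistics panel.
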(event `self.ReceiveBeginPlay`
  (bind _returnvalue (`|SpawnActorFromClass` "/Game/Core/Controllers/AICon_TBS_AIController.AICon_TBS_AIController_C" (`KismetMathLibrary.MakeTransform` (0.0 0.0 0.0)) "Undefined" "OverrideRootScale" null null)) ; Spawn AI Controller
  (set `self.AI Controller` _returnvalue)
  (bind _returnvalue_2 (`|SpawnActorFromClass` "/Game/Blueprints/BP_TBS_RoomManager.BP_TBS_RoomManager_C" (`KismetMathLibrary.MakeTransform` (0.0 0.0 0.0)) "Undefined" "OverrideRootScale" null null)) ; Spawn Room Manager
  (set `self.Room Manager` _returnvalue_2)
  ;[1 1 1] DEBUG HUD Setup
  (bind _returnvalue_3 (`|CreateWidget` "/Game/UI/DebugScreen.DebugScreen_C")) ; DEBUG WIDGET
  (bind _output_get (set `self.[DEBUG] Widget` _returnvalue_3))
  (`|ExecutionSequence`
    (:`then_0`
      (`UserWidget.AddToViewport` _output_get 0))
    (:`then_1`
      (bind _returnvalue_4 (`|CreateWidget` "/Game/UI/DEBUG_StatDisplay.DEBUG_StatDisplay_C" null "Room Manager" (`KismetTextLibrary.Conv_StringToText` (`KismetSystemLibrary.GetDisplayName` (`self.Room Manager`)))))
      (`PanelWidget.AddChild` (`/Game/UI/DebugScreen.StatisticsPanel` _output_get) _returnvalue_4))))

(fn `UserConstructionScript`)