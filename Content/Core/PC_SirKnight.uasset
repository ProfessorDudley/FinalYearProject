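; Player controller for a grid-based Munchkin card game that handles click-to-move, drawing cards into the pawn's hand and hand UI updates.
; Left-click traces under the cursor and runs a hand-written, Dijkstra-like search over the current room's tiles, scored by distance from the origin.
; Parent links yield a target-to-origin path, which ExecuteMoveTo walks backwards with short delays.
; End Turn only prints, with turn advancement disconnected.
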(event `Key|LeftMouseButton`
  (params (Key :type "Key Structure"))
  (bind (_hitresult _returnvalue) (`self.GetHitResultUnderCursorByChannel` "TraceTypeQuery3"))
  (bind _current_room (`/Game/Core/GM_Munchkin.Current Room` (`self.Gamemode`)))
  (:`Pressed`
    (if _returnvalue
      (bind _out_steps (`self.Literally just Pathfinding` (`/Game/Pawns/Pawn_ParentUnit.Coordinate` (`self.Controlled Pawn`)) (`/Game/Core/Macros_PC_SirKnight.Location to Coordinates` (`.Location` (`GameplayStatics.BreakHitResult` _hitresult))) (`/Game/Blueprints/BP_Room.Grid Coordinates` _current_room) (`/Game/Blueprints/BP_Room.Room Template` _current_room))) ; Currently outputs only the direct path. Need to add all nearest tiles.
      (for _array_element _out_steps
        (`KismetSystemLibrary.PrintString` (`KismetStringLibrary.Conv_Vector2dToString` _array_element) true true (struct :`B` 1.0 :`A` 1.0) 3.0))
      (`self.Execute MoveTo` (`self.Controlled Pawn`) _out_steps))))

(event `Key|RightMouseButton`
  (params (Key :type "Key Structure")))

(event `self.ReceiveBeginPlay`
  (`|ExecutionSequence`
    (:`then_0`
      (set `self.Gamemode` (cast `/Game/Core/GM_Munchkin` (`GameplayStatics.GetGameMode`) :!pure true))
      (`KismetSystemLibrary.PrintString` (`KismetSystemLibrary.GetDisplayName` (`GameplayStatics.GetPlayerController` 0)) true true (struct :`R` 1.0 :`G` 0.5 :`A` 1.0)))
    (:`then_1`
      (set `self.bShowMouseCursor` true)
      (`WidgetBlueprintLibrary.SetInputMode_GameAndUIEx` self))))

(event `Assign UI Inputs to Actions`
  (`|ExecutionSequence`
    (:`then_0`
      (add `/Game/UI/Screens/Screen_Combat.Event End Turn` (`self.HUD Reference`) (delegate `Event End Turn_Event_0`)))))

(event `Event End Turn_Event_0`
  (`KismetSystemLibrary.PrintString` "Event End Turn" true true (struct :`R` 1.0 :`G` 0.358091 :`A` 1.0)))

(fn `Draw Card`
  (params (Index :type Integer) (`Game Deck` :type "Array of /Game/Blueprints/Struct_Card Structure"))
  (returns (ReturnValue :type Boolean))
  (bind _returnvalue (`KismetArrayLibrary.Array_IsValidIndex` `Game Deck` Index))
  (bind _hand (`/Game/Pawns/Pawn_ParentUnit.Hand` (`self.Controlled Pawn`)))
  (if _returnvalue
    (bind _returnvalue_2 (`KismetArrayLibrary.Array_Add` _hand (`|GetArrayItem` `Game Deck` Index)))
    (`KismetArrayLibrary.Array_Remove` `Game Deck` Index)
    (`KismetSystemLibrary.PrintString` (`KismetStringLibrary.Concat_StrStr` "\"" (`KismetTextLibrary.Conv_TextToString` (`.Name_2_180633DC47C824C3FB7B2CBED7904891` (break `/Game/Blueprints/Struct_Card` (`|GetArrayItem` _hand _returnvalue_2)))) "\" was removed from the Deck and added to the hand.") false true (struct :`R` 0.5 :`B` 1.0 :`A` 1.0))
    (return _returnvalue)
    (else
      (`KismetSystemLibrary.PrintString` "Unable to Draw Card" true true (struct :`R` 1.0 :`A` 1.0))
      (return _returnvalue))))

(fn `Literally just Pathfinding`
  (params (CurrentTile :type "Vector2D Structure") (Target :type "Vector2D Structure") (`World Grid` :type "Array of Vector2D Structure") (`Tile Grid` :type "Map of Vector2D Structure to /Game/Blueprints/Struct_RoomGrid Structure") (Range :type Integer))
  (returns (`Out Steps` :type "Array of Vector2D Structure"))
  (locals (`[LOCAL] Origin` :type "Vector2D Structure") (`[LOCAL] OpenList` :type "Map of Vector2D Structure to /Game/Blueprints/Struct_TileCost Structure") (`[LOCAL] Closed List` :type "Array of Vector2D Structure") (`[LOCAL] Current Tile` :type "Vector2D Structure") (`[LOCAL] Scores Array` :type "Array of Integer") (`[LOCAL] Searching` :type Boolean :default true) (`[LOCAL] Tile Steps` :type "Array of Vector2D Structure") (`[LOCAL] Iterations` :type Integer) (`[LOCAL] Min Index` :type Integer :default 0) (`[LOCAL] World Grid` :type "Array of Vector2D Structure") (`[LOCAL] Target` :type "Vector2D Structure") (`[LOCAL] Tile Grid` :type "Map of Vector2D Structure to /Game/Blueprints/Struct_RoomGrid Structure"))
  (bind __local__current_tile (`local.[LOCAL] Current Tile`))
  (bind __local__scores_array (`local.[LOCAL] Scores Array`))
  (bind __local__openlist (`local.[LOCAL] OpenList`))
  (bind _value (`BlueprintMapLibrary.Map_Find` (`local.[LOCAL] OpenList`) (`local.[LOCAL] Current Tile`)))
  ;[0 0.03172 1] Initialising variables.
  (`|ExecutionSequence`
    (:`then_0`
      (set `local.[LOCAL] Tile Grid` `Tile Grid`)
      (bind _output_get (set `local.[LOCAL] World Grid` `World Grid`))
      (set `local.[LOCAL] Target` Target)
      (bind _output_get_2 (set `local.[LOCAL] Origin` CurrentTile))
      (bind _output_get_3 (set `local.[LOCAL] Current Tile` _output_get_2))
      (`BlueprintMapLibrary.Map_Add` (`local.[LOCAL] OpenList`) _output_get_3 (make `/Game/Blueprints/Struct_TileCost` (`/Game/Core/Functions_Pathfinding.Coords -> Index` _output_get_3 _output_get) 0 _output_get_3)))
    (:`then_1`
      ;[0.2202 0 1] Restart from Here!
      (for (_ _array_index) (`local.[LOCAL] World Grid`)
        (`KismetArrayLibrary.Array_Clear` (`local.[LOCAL] Scores Array`))
        (set `local.[LOCAL] Iterations` _array_index)
        (bind (_found_coordinates _coordinates) (`/Game/Core/Functions_Pathfinding.Get Multiple Adjacent Coordinates` (`local.[LOCAL] Current Tile`) (`local.[LOCAL] World Grid`) (`local.[LOCAL] Tile Grid`))) ; Find the walkable tiles around the current tile
        (if _found_coordinates
          ;[1 1 1] Calculate a tile's distance from the origin and add it to the open list map. Also make note of it's parent.
          (for _array_element _coordinates
            (if (not (`KismetArrayLibrary.Array_Contains` (`local.[LOCAL] Closed List`) _array_element))
              (bind _distance (`/Game/Core/Functions_Pathfinding.Get Distance to Target` (`local.[LOCAL] Origin`) _array_element)) ; Get it's distance from the origin tile (Cost)
              (`BlueprintMapLibrary.Map_Add` (`local.[LOCAL] OpenList`) _array_element (make `/Game/Blueprints/Struct_TileCost` (`/Game/Core/Functions_Pathfinding.Coords -> Index` _array_element (`local.[LOCAL] World Grid`)) _distance (`local.[LOCAL] Current Tile`))) ; Add to the open list with it's tile cost and parent tile
            ))
          ;[1 1 1] Check if we have not found the target.
          (`KismetArrayLibrary.Array_AddUnique` (`local.[LOCAL] Closed List`) __local__current_tile)
          (if (!= __local__current_tile (`local.[LOCAL] Target`))
            ;[1 1 1] Add all the tiles in the open list's scores to an array for sorting.
            (bind _values (`BlueprintMapLibrary.Map_Values` __local__openlist))
            (for _array_element_2 _values
              (`KismetArrayLibrary.Array_Add` __local__scores_array (`.Cost_6_2880D152496ED1988E23E0A66CC06617` (break `/Game/Blueprints/Struct_TileCost` _array_element_2))))
            ;[1 1 1] Find the tile with the lowest cost and set it as the current tile. Restart the for each loop.
            (bind _keys (`BlueprintMapLibrary.Map_Keys` __local__openlist))
            (bind _output_get_4 (set `local.[LOCAL] Min Index` (`KismetMathLibrary.MinOfIntArray` __local__scores_array)))
            (bind _output (`|GetArrayItem` _keys _output_get_4))
            (if (`KismetArrayLibrary.Array_Contains` (`local.[LOCAL] Closed List`) _output) :!label _label
              (bind _output_get_5 (set `local.[LOCAL] Min Index` (+ (stale _output_get_5) 1)))
              (goto _label)
              (else
                (set `local.[LOCAL] Current Tile` _output)))
            (else
              (break)))))
      ;[1 1 1] Get the tiles that make up the shortest path for the pawn to move across.
      (for _ (range 49)
        (`KismetArrayLibrary.Array_AddUnique` (`local.[LOCAL] Tile Steps`) (`local.[LOCAL] Current Tile`)) ; Add tiles to the output array
        (set `local.[LOCAL] Current Tile` (`.Parent_8_BFC9374742AD9EA520DA9E81098B7EED` (break `/Game/Blueprints/Struct_TileCost` _value)))
        (if (== (`.Cost_6_2880D152496ED1988E23E0A66CC06617` (break `/Game/Blueprints/Struct_TileCost` _value)) 0)
          (break)))
      (return (`local.[LOCAL] Tile Steps`)) ; Exit. Please make it stop.
    )))

(fn `Update Hand`
  (`self.UI Update Hand` (`/Game/Pawns/Pawn_ParentUnit.Hand` (`self.Controlled Pawn`))))

(fn `UserConstructionScript`)